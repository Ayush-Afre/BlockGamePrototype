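; BP_Block is a breakable block actor that can be destroyed over time and collected into the player's inventory.
; On BeginPlay it creates a dynamic material and sets the destroy timeline's play rate from DestroyRate.
; StartDestroy drives the material's DestroyAmount through the timeline, while StopDestroy halts and resets it.
; When the timeline finishes, it removes itself from GI_BlockGame by location, adds its class to BP_FirstPersonCharacter's inventory and destroys itself.
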(event Custom|StartDestroy
  ;[0.125 0.125 0.125] Edit the dynamic material to start or stop a destroy
  (bind _destroyamount (Timeline|DestroyTimeline PlayFromStart)
    (:Update
      (Rendering|Material|SetScalarParameterValue (Variables|Default|GetBlockMat) "DestroyAmount" _destroyamount :!class /Script/Engine.MaterialInstanceDynamic))
    (:Finished
      (Default|RemoveBlock (.AsGI%20Block%20Game (Utilities|Casting|CastToGI_BlockGame (Game|GetGameInstance))) (Transformation|GetWorldLocation (Variables|Default|GetDefaultSceneRoot)))
      (bind _asbp_first_person_character (Utilities|Casting|CastToBP_FirstPersonCharacter (Game|GetPlayerCharacter 0))
        (:then
          (Default|AddBlocktoInventory _asbp_first_person_character (Utilities|GetClass self)))
        (:CastFailed
          _))
      (Actor|DestroyActor))))

(event Custom|StopDestroy
  ;[0.125 0.125 0.125] Edit the dynamic material to start or stop a destroy
  (Rendering|Material|SetScalarParameterValue (Variables|Default|GetBlockMat) "DestroyAmount" 0.0 :!class /Script/Engine.MaterialInstanceDynamic) ; Reseting the destroy parameter
  (bind _destroyamount (Timeline|DestroyTimeline Stop)
    (:Update
      (Rendering|Material|SetScalarParameterValue (Variables|Default|GetBlockMat) "DestroyAmount" _destroyamount :!class /Script/Engine.MaterialInstanceDynamic))
    (:Finished
      (Default|RemoveBlock (.AsGI%20Block%20Game (Utilities|Casting|CastToGI_BlockGame (Game|GetGameInstance))) (Transformation|GetWorldLocation (Variables|Default|GetDefaultSceneRoot)))
      (bind _asbp_first_person_character (Utilities|Casting|CastToBP_FirstPersonCharacter (Game|GetPlayerCharacter 0))
        (:then
          (Default|AddBlocktoInventory _asbp_first_person_character (Utilities|GetClass self)))
        (:CastFailed
          _))
      (Actor|DestroyActor))))

(event EventBeginPlay
  (bind _block (Variables|Default|GetBlock))
  ;[0.02604 0.02604 0.02604] Begin Play - Create a dynamic material and set hte play rate
  (bind _returnvalue (Rendering|Material|CreateDynamicMaterialInstance _block 0 (Rendering|Material|GetMaterial _block 0) "None" :!class /Script/Engine.PrimitiveComponent))
  (Variables|Default|SetBlockMat _returnvalue)
  (Components|Timeline|SetPlayRate (Variables|Default|GetDestroyTimeline) (Variables|Default|GetDestroyRate)))

(fn ConstructionScript)