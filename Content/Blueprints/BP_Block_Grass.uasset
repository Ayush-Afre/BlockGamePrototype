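; BP_Block_Grass is a breakable grass block for a block-based game that goes into the player's inventory when destroyed.
; BeginPlay creates dynamic material instances for three material slots and scales the timeline's play rate by DestroyRate.
; StartDestroy runs a timeline driving each material's DestroyAmount, while StopDestroy halts it and resets the effect.
; On completion, it removes its location from GI_BlockGame, gives its class to BP_FirstPersonCharacter and destroys itself.
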(event EventBeginPlay
  (bind _block (Variables|Default|GetBlock))
  (Components|Timeline|SetPlayRate (Variables|Default|GetDestroyTimeline) (Variables|Default|GetDestroyRate))
  (for _index (range 0 2)
    (bind _returnvalue (Rendering|Material|CreateDynamicMaterialInstance _block _index (Rendering|Material|GetMaterial _block _index) "None" :!class /Script/Engine.PrimitiveComponent))
    (Utilities|Array|Add (Variables|Default|GetMaterials) _returnvalue)))

(event EventStartDestroy
  (bind _destroyamount (Timeline|Timeline PlayFromStart)
    (:Update
      (Rendering|Material|SetScalarParameterValue (Variables|Default|GetMaterials) "DestroyAmount" _destroyamount :!class /Script/Engine.MaterialInstanceDynamic))
    (:Finished
      (Default|RemoveBlock (.AsGI%20Block%20Game (Utilities|Casting|CastToGI_BlockGame (Game|GetGameInstance))) (Transformation|GetWorldLocation (Variables|Default|GetDefaultSceneRoot)))
      (bind _asbp_first_person_character (Utilities|Casting|CastToBP_FirstPersonCharacter (Game|GetPlayerCharacter 0))
        (:then
          (Default|AddBlocktoInventory _asbp_first_person_character (Utilities|GetClass self)))
        (:CastFailed
          _))
      (Actor|DestroyActor))))

(event EventStopDestroy
  (Rendering|Material|SetScalarParameterValue (Variables|Default|GetMaterials) "DestroyAmount" 0.0 :!class /Script/Engine.MaterialInstanceDynamic)
  (bind _destroyamount (Timeline|Timeline Stop)
    (:Update
      (Rendering|Material|SetScalarParameterValue (Variables|Default|GetMaterials) "DestroyAmount" _destroyamount :!class /Script/Engine.MaterialInstanceDynamic))
    (:Finished
      (Default|RemoveBlock (.AsGI%20Block%20Game (Utilities|Casting|CastToGI_BlockGame (Game|GetGameInstance))) (Transformation|GetWorldLocation (Variables|Default|GetDefaultSceneRoot)))
      (bind _asbp_first_person_character (Utilities|Casting|CastToBP_FirstPersonCharacter (Game|GetPlayerCharacter 0))
        (:then
          (Default|AddBlocktoInventory _asbp_first_person_character (Utilities|GetClass self)))
        (:CastFailed
          _))
      (Actor|DestroyActor))))

(fn ConstructionScript
  (|CallParentFunction))